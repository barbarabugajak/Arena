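; Screen tint handler that gives feedback on player damage, healing and low health through a post-process volume.
; On BeginPlay it clears the tint and binds player events that swap the volume's material between red and green and toggle its blend weight.
; Damage flashes red, healing flashes green, and low health blinks the tint in a Delay loop until the low-health-off event clears the blink flag.
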(event `self.ReceiveBeginPlay`
  ; Initially Disable Tint. Bind Events
  (`self.SetTint` 0.0)
  (add `self.PlayerDamage` (delegate `PlayerDamage_Event`))
  (add `self.PlayerLowHealthOn` (delegate `LowHealthOn`))
  (add `self.PlayerLowHealthOff` (delegate `PlayerLowHealthOff_Event`))
  (add `self.PlayerIsHealing` (delegate `PlayerHeal_Event`)))

(event `PlayerHeal_Event`
  ; Green Tint on Heal
  (`self.Set Color` true)
  (`self.SetTint` 1.0)
  (`KismetSystemLibrary.Delay` 0.3)
  (`self.SetTint` 0.0)
  (`self.Set Color` false))

(event `PlayerDamage_Event`
  ; Enable Tint on Player Low Health
  (`self.Set Color` false)
  (`self.SetTint` 1.0)
  (`KismetSystemLibrary.Delay` 0.2)
  (`self.SetTint` 0.0))

(event `PlayerLowHealthOff_Event`
  ; Disable Tint
  (set `self.bShouldBlink` false))

(event `LowHealthOn`
  ; Blink Tint
  (`self.Set Color` false)
  (set `self.bShouldBlink` true)
  (`KismetSystemLibrary.Delay` 0.2 :!label _label)
  (`self.SetTint` 1.0)
  (`KismetSystemLibrary.Delay` 0.2)
  (`self.SetTint` 0.0)
  (if (`self.bShouldBlink`)
    (goto _label)))

(fn `Set Color`
  (params (`Set to green` :type Boolean))
  (bind _array (break `WeightedBlendables` (`.WeightedBlendables` (break `PostProcessSettings` (`PostProcessVolume.Settings` (`self.PostProcessVolumeRef`))))))
  (if `Set to green`
    (`KismetArrayLibrary.Array_Set` _array 0 (make `WeightedBlendable` 1.0 (`self.Material_Green`)))
    (else
      (`KismetArrayLibrary.Array_Set` _array 0 (make `WeightedBlendable` 1.0 (`self.Material_Red`))))))

(fn `SetTint`
  (params (`Blend Weight` :type "Float (single-precision)"))
  (set `PostProcessVolume.BlendWeight` `Blend Weight` (`self.PostProcessVolumeRef`)))

(fn `UserConstructionScript`)