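; BP_Wizard_Dark is a dark wizard enemy that reports to the player character's WaveSpawner when destroyed.
; Its damage event briefly flashes a mesh overlay material chosen by Melee, Magic or Fire type, and shows an animated damage indicator, currently passed zero rather than the actual amount.
; Tick updates the health widget's progress bar from Health over MaxHealth.
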(event `self.ReceiveBeginPlay`
  ; BeginPlay()
  ;; Assign WaveSpawner references
  (bind _asbp_character (cast `/Game/BP/BP_Character` (`GameplayStatics.GetPlayerCharacter` 0)))
  (set `self.BP Enemy Spawner` (`/Game/BP/BP_Character.Wave Spawner` _asbp_character))
  ;; Bind Damage Indicator
  (add `self.IndicateDamageDelegate` (delegate `IndicateDamage_Event`))
  (`SceneComponent.SetVisibility` (`self.DamageIndicatorWidget`) false true))

(event `IndicateDamage_Event`
  (params (DamageAmount :type "Float (single-precision)") (DamageType :type String))
  (bind _mesh (`self.Mesh`))
  ; Add overlay material for each damage type
  (`KismetSystemLibrary.PrintString` DamageType)
  (`self.DisplayDamageIndicator` 0.0)
  (switch `string` DamageType
    (:`Melee`
      (set `self.CurrentOverlayMat` "/Game/PortalMaterial/Material/MM/M_Red_Inst.M_Red_Inst"))
    (:`Magic`
      (set `self.CurrentOverlayMat` "/Game/PortalMaterial/Material/M_Wisp_Inst1.M_Wisp_Inst1"))
    (:`Fire`
      (set `self.CurrentOverlayMat` "/Game/PortalMaterial/Material/MM/M_Wisp_Inst.M_Wisp_Inst")))
  (`MeshComponent.SetOverlayMaterial` _mesh (`self.CurrentOverlayMat`))
  (`KismetSystemLibrary.Delay` 0.2)
  (`MeshComponent.SetOverlayMaterial` _mesh null))

(event `self.ReceiveTick`
  (params (DeltaSeconds :type "Float (single-precision)"))
  ; Update Health Widget
  (bind _asbp_health_enemy (cast `/Game/UI/BP_HealthEnemy` (`WidgetComponent.GetWidget` (`self.Widget`))))
  (`/Engine/EditorBlueprintResources/StandardMacros.IsValid` _asbp_health_enemy
    (:`Is Valid`
      (`ProgressBar.SetPercent` (`/Game/UI/BP_HealthEnemy.ProgressBar_13` _asbp_health_enemy) (`KismetMathLibrary.SafeDivide` (`self.Health`) (`self.MaxHealth`))))))

(event `self.ReceiveDestroyed`
  ; Update Enemy Spawner Count on Destruction
  (`/Engine/EditorBlueprintResources/StandardMacros.IsValid` (`self.BP Enemy Spawner`)
    (:`Is Valid`
      (`/Game/BP/Waves/BP_Wave_Spawner.EnemyDead` (`self.BP Enemy Spawner`)))
    (:`Is Not Valid`
      (bind _asbp_character (cast `/Game/BP/BP_Character` (`GameplayStatics.GetPlayerCharacter` 0)))
      (`/Game/BP/Waves/BP_Wave_Spawner.EnemyDead` (`/Game/BP/BP_Character.Wave Spawner` _asbp_character)))))

(fn `DisplayDamageIndicator`
  (params (`Damage Amount` :type "Float (double-precision)"))
  (bind _damageindicatorwidget (`self.DamageIndicatorWidget`))
  (bind _asbp_damage_indicator (cast `/Game/UI/BP_DamageIndicator` (`WidgetComponent.GetWidget` _damageindicatorwidget)))
  (`SceneComponent.SetVisibility` _damageindicatorwidget true true)
  (set `TextBlock.Text` (`KismetTextLibrary.Conv_DoubleToText` `Damage Amount` "HalfToEven") (`/Game/UI/BP_DamageIndicator.DamageText` _asbp_damage_indicator))
  (`/Game/UI/BP_DamageIndicator.PlayAnim` _asbp_damage_indicator))

(fn `UserConstructionScript`)