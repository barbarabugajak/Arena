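; BP_DarkWizard is an enemy wizard that displays its health on a widget and reports its death to the wave spawner.
; On BeginPlay it stores the first BP_WaveSpawner found in the level.
; Every Tick it casts its widget to BP_HealthEnemy and sets the progress bar to Health over MaxHealth.
; When destroyed, it calls EnemyDead on the spawner and prints a debug message.
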(event `self.ReceiveBeginPlay`
  (bind _outactors (`GameplayStatics.GetAllActorsOfClass` "/Game/BP/Waves/BP_WaveSpawner.BP_WaveSpawner_C"))
  (set `self.BP Enemy Spawner` (`|GetArrayItem` _outactors)))

(event `self.ReceiveTick`
  (params (DeltaSeconds :type "Float (single-precision)"))
  (bind _asbp_health_enemy (cast `/Game/UI/BP_HealthEnemy` (`WidgetComponent.GetWidget` (`self.Widget`))))
  (`/Engine/EditorBlueprintResources/StandardMacros.IsValid` _asbp_health_enemy
    (:`Is Valid`
      (`ProgressBar.SetPercent` (`/Game/UI/BP_HealthEnemy.ProgressBar_13` _asbp_health_enemy) (`KismetMathLibrary.SafeDivide` (`self.Health`) (`self.MaxHealth`))))))

(event `self.ReceiveDestroyed`
  (`/Game/BP/Waves/BP_WaveSpawner.EnemyDead` (`self.BP Enemy Spawner`))
  (`KismetSystemLibrary.PrintString` "DarkWizard: Destroyes"))

(fn `UserConstructionScript`)