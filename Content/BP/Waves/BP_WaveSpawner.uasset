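; Wave spawner actor that spawns enemy waves from an array of wave data assets and triggers the player character's Win once waves run out.
; SpawnNewWave spawns each entry's enemy type and count at random BP_SpawnLocation actors, incrementing CurrentWave inside the per-enemy loop.
; EnemyDead decrements the remaining count and requests another wave at zero.
; BeginPlay only sets the last wave index, so ShouldSpawnNewWave drives spawning.
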(event `ShouldSpawnNewWave`
  (`self.SpawnNewWave`))

(event `self.ReceiveBeginPlay`
  (bind _output_get (set `self.MaxWaves` (`KismetArrayLibrary.Array_Length` (`self.WaveData`))))
  (`/Engine/EditorBlueprintResources/StandardMacros.DecrementInt` _output_get))

(event `EnemyDead`
  (bind _enemies_left (`self.Enemies Left`))
  (`/Engine/EditorBlueprintResources/StandardMacros.DecrementInt` _enemies_left
    (:`  `
      (`KismetSystemLibrary.PrintString` (`KismetStringLibrary.Conv_IntToString` _enemies_left))
      (if (<= _enemies_left 0)
        (`self.ShouldSpawnNewWave`)))))

(fn `SpawnNewWave`
  (locals (AllSpawnLocs :type "Array of /Game/BP/Waves/BP_SpawnLocation Object Reference"))
  (bind _allspawnlocs (`local.AllSpawnLocs`))
  (set `self.Enemies Left` 1)
  (if (<= (`self.Current Wave`) (`self.MaxWaves`))
    (bind _output_get (set `self.Current Wave Data Asset` (`|GetArrayItem` (`self.WaveData`) (`self.Current Wave`))))
    (bind _outactors (`GameplayStatics.GetAllActorsOfClass` "/Game/BP/Waves/BP_SpawnLocation.BP_SpawnLocation_C"))
    (set `local.AllSpawnLocs` _outactors)
    (for _array_element (`/Game/BP/Waves/BP_WaveDataAsset.WaveData` _output_get)
      (set `self.Enemies Left` (+ (`.HowManyEnemies_10_4B71784F0D439435C6CA88BAC7844743` (break `/Game/BP/Waves/BP_WaveEnemyInfo_Struct` _array_element)) (`self.Enemies Left`)))
      (for _ (range (+ (`.HowManyEnemies_10_4B71784F0D439435C6CA88BAC7844743` (break `/Game/BP/Waves/BP_WaveEnemyInfo_Struct` _array_element)) 1))
        (`|SpawnActorFromClass` (`.TypeOfEnemy_7_51595241BE4A7F8173E5C78337B81590` (break `/Game/BP/Waves/BP_WaveEnemyInfo_Struct` _array_element)) (`KismetMathLibrary.MakeTransform` (`self.K2_GetActorLocation` (`|GetArrayItem` _allspawnlocs (`KismetMathLibrary.RandomInteger` (`KismetArrayLibrary.Array_Length` _allspawnlocs))))) "Undefined" "MultiplyWithRoot" null null)
        (set `self.Current Wave` (+ 1 (`self.Current Wave`)))))
    (else
      (bind _asbp_character (cast `/Game/BP/BP_Character` (`GameplayStatics.GetPlayerCharacter` 0)))
      (`/Game/BP/BP_Character.Win` _asbp_character))))

(fn `UserConstructionScript`)