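; BP_Wave_Spawner runs enemy waves defined by an ordered list of wave data assets and triggers the player's win once all are done.
; SpawnNewWave reads the current asset's enemy types and counts, spawning each enemy at a random BP_SpawnLocation actor.
; EnemyDead decrements the remaining count and starts the next wave at zero.
; After the last wave, it calls Win on a living BP_Character.
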(event `ShouldSpawnNewWave`
  ; Spawn new wave
  (`self.SpawnNewWave`))

(event `self.ReceiveBeginPlay`
  ; Set Max Waves to Length of Wave Data
  (bind _output_get (set `self.MaxWaves` (`KismetArrayLibrary.Array_Length` (`self.WaveData`))))
  (`/Engine/EditorBlueprintResources/StandardMacros.DecrementInt` _output_get))

(event `EnemyDead`
  (bind _enemies_left (`self.Enemies Left`))
  ; On Enemy Death decrease Enemies Left, check if Spawn New Wave
  (`/Engine/EditorBlueprintResources/StandardMacros.DecrementInt` _enemies_left
    (:`  `
      (if (<= _enemies_left 0)
        (`self.ShouldSpawnNewWave`)))))

(fn `SpawnNewWave`
  (locals (AllSpawnLocs :type "Array of /Game/BP/Waves/BP_SpawnLocation Object Reference"))
  (bind _allspawnlocs (`local.AllSpawnLocs`))
  (set `self.Enemies Left` 0)
  (if (<= (`self.Current Wave`) (`self.MaxWaves`))
    (bind _output_get (set `self.Current Wave Data Asset` (`|GetArrayItem` (`self.WaveData`) (`self.Current Wave`))))
    (bind _outactors (`GameplayStatics.GetAllActorsOfClass` "/Game/BP/Waves/BP_SpawnLocation.BP_SpawnLocation_C"))
    (set `local.AllSpawnLocs` _outactors)
    (for _array_element (`/Game/BP/Waves/BP_Wave_DataAsset.WaveData` _output_get)
      (set `self.Enemies Left` (+ (`.HowManyEnemies_10_4B71784F0D439435C6CA88BAC7844743` (break `/Game/BP/Waves/BP_Wave_Enemy_Info_Struct` _array_element)) (`self.Enemies Left`)))
      (for _ (range 1 (+ (`.HowManyEnemies_10_4B71784F0D439435C6CA88BAC7844743` (break `/Game/BP/Waves/BP_Wave_Enemy_Info_Struct` _array_element)) 1))
        (`|SpawnActorFromClass` (`.TypeOfEnemy_11_51595241BE4A7F8173E5C78337B81590` (break `/Game/BP/Waves/BP_Wave_Enemy_Info_Struct` _array_element)) (`KismetMathLibrary.MakeTransform` (`self.K2_GetActorLocation` (`|GetArrayItem` _allspawnlocs (`KismetMathLibrary.RandomInteger` (`KismetArrayLibrary.Array_Length` _allspawnlocs))))) "Undefined" "MultiplyWithRoot" null null)))
    (set `self.Current Wave` (+ 1 (`self.Current Wave`)))
    (else
      (bind _asbp_character (cast `/Game/BP/BP_Character` (`GameplayStatics.GetPlayerCharacter` 0)))
      (if (`PlayerCharacter.bIsAlive` _asbp_character)
        (`/Game/BP/BP_Character.Win` _asbp_character)
        (else
          (`KismetSystemLibrary.PrintString` "Died, no UI"))))))

(fn `UserConstructionScript`)