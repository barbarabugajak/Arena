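; BP_Ray is a timed ray actor that shows a highlight before the ray appears and becomes collidable.
; It starts hidden without collision and waits for its OnSpawned event, which supplies the delay between highlight and ray.
; When the delay ends, it swaps highlight for mesh, enables collision and plays a sound.
; A timeline then animates the box component's uniform world scale, and the actor destroys itself when finished.
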(event `self.ReceiveBeginPlay`
  ; Hide ray and disable collision on spawn
  (`self.SetActorEnableCollision` false)
  (`SceneComponent.SetVisibility` (`self.BoxComponent`) false true)
  ; Ray Animation & Collision
  (add `self.OnSpawned` (delegate `OnSpawned_Event`)))

(event `OnSpawned_Event` :!signature `self.OnSpawned`
  (params (Delay :type "Float (single-precision)"))
  ; Ray Animation & Collision
  (`SceneComponent.SetVisibility` (`self.Highlight`) true false) ; Show Highlight
  (`KismetSystemLibrary.Delay` Delay)
  (`SceneComponent.SetVisibility` (`self.StaticMesh`) true false) ; Show Ray itself
  (`SceneComponent.SetVisibility` (`self.Highlight`) false false) ; Hide Highlight (Ray is visible now)
  (`self.SetActorEnableCollision` true) ; Enable Ray Collision
  (`GameplayStatics.PlaySound2D` "/Game/Assets/Sound/elemental-magic-spell-impact-outgoing-228342.elemental-magic-spell-impact-outgoing-228342" 0.5 1.0 0.0 null null)
  (bind (_direction _ray_radius) (`Timeline|Timeline`) ; Ray size animation
    (:`Update`
      (`SceneComponent.SetWorldScale3D` (`self.BoxComponent`) (`KismetMathLibrary.MakeVector` _ray_radius _ray_radius _ray_radius)))
    (:`Finished`
      (`self.K2_DestroyActor`))))

(fn `UserConstructionScript`)